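; Truck camera component that applies the Better Vehicle Camera mod config to the owning BP_Truck's spring arm and camera.
; UpdateCameraValues sets lag, arm length and offsets from stored base transforms, then resets zoom.
; It runs on any change to a main-category setting, and via a Tick check when player control begins outside vehicle or train first-person mode.
; Optional zoom inputs step the arm length within clamped limits.
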(event Custom|GetTruckReferences
  ;[1 1 1] Get Owner References
  (bind _asbp_truck (Utilities|Casting|CastToBP_Truck (Components|GetOwner)))
  (bind _output_get (Variables|OwnerReferences|SetOwner _asbp_truck))
  (Variables|OwnerReferences|SetOwnerCamera (Variables|/Game/FactoryGame/Buildable/Vehicle/Truck/BP_Truck.BP_Truck_C|GetCamera _output_get))
  (Variables|OwnerReferences|SetOwnerSpringArm (Variables|/Game/FactoryGame/Buildable/Vehicle/Truck/BP_Truck.BP_Truck_C|GetSpringArm _output_get)))

(event Custom|ResetCameraZoom
  ;[1 1 1] Reset Camera zoom
  (Variables|CameraZoom|SetCameraZoom (Class|RuntimeBlueprintFunctionLibrary|ToFloat(ConfigProperty) (Class|RuntimeBlueprintFunctionLibrary|ToConfigProperty(ConfigPropertySection) (.AsConfig%20Property%20Section (Utilities|Casting|CastToConfigPropertySection (Class|RuntimeBlueprintFunctionLibrary|ToConfigProperty(ConfigPropertySection) (.AsConfig%20Property%20Section (Utilities|Casting|CastToConfigPropertySection (Class|RuntimeBlueprintFunctionLibrary|ToConfigProperty(ConfigPropertySection) (.AsBP%20Config%20Property%20Section (Utilities|Casting|CastToBP_ConfigPropertySection (Class|RuntimeBlueprintFunctionLibrary|ToConfigProperty(ModConfiguration) "/BetterVehicleCamera/Config/BetterVehicleCamera_Config.BetterVehicleCamera_Config_C"))) (Variables|Default|GetMainSettingsCategory)))) "SpringArmPosition"))) "SpringArmLength"))))

(event Custom|AssignUpdateEvent
  ;[1 1 1] Update Camera Position when settings changed
  (bind _asbp_config_property_section (Utilities|Casting|CastToBP_ConfigPropertySection (Class|RuntimeBlueprintFunctionLibrary|ToConfigProperty(ModConfiguration) "/BetterVehicleCamera/Config/BetterVehicleCamera_Config.BetterVehicleCamera_Config_C")))
  (bind _asconfig_property_section (Utilities|Casting|CastToConfigPropertySection (Class|RuntimeBlueprintFunctionLibrary|ToConfigProperty(ConfigPropertySection) _asbp_config_property_section (Variables|Default|GetMainSettingsCategory))))
  (bind _values (Utilities|Map|Values (Variables|/Script/SML.ConfigPropertySection|GetSectionProperties _asconfig_property_section)))
  (for _array_element _values
    (bind _asconfig_property_section_2 (Utilities|Casting|CastToConfigPropertySection _array_element))
    (bind _values_2 (Utilities|Map|Values (Variables|/Script/SML.ConfigPropertySection|GetSectionProperties _asconfig_property_section_2)))
    (for _array_element_2 _values_2
      (EventDispatchers|BindEventtoOnPropertyValueChanged _array_element_2 (delegate Custom|UpdateCameraValues)))))

(event Custom|ZoomValueChanged
  ;[1 1 1] Update Camera arm length according to zoom
  (Variables|/Script/Engine.SpringArmComponent|SetTargetArmLength (Variables|OwnerReferences|GetOwnerSpringArm) (Variables|CameraZoom|GetCameraZoom)))

(event Custom|PlayerControlBasedUpdate
  ;[1 1 1] Check if player is in vehicle and not currently in first person with compatible mods
  (bind _output_get (Variables|PlayerControlStatus|SetIsPlayerControlled (Pawn|IsPlayerControlled (Variables|OwnerReferences|GetOwner))))
  (if _output_get
    (if (not (or (Variables|/FirstPersonVehicles/BP_FirstPersonVehicles_VehicleCameraSwitchSubsystem.BP_FirstPersonVehicles_VehicleCameraSwitchSubsystem_C|GetVehicleFirstPersonActive (Variables|CompatibleSubsystems|GetFirstPersonVehiclesSubsystem)) (Variables|/TrainInteriors/BP_TrainInteriors_TrainCameraSwitchSubsystem.BP_TrainInteriors_TrainCameraSwitchSubsystem_C|GetTrainFirstPersonActive (Variables|CompatibleSubsystems|GetTrainInteriorSubsystem))))
      (if (not (stale _output_get_2))
        (CallFunction|UpdateCameraValues)
        (Variables|PlayerControlStatus|SetWasPlayerControlled true)))
    (else
      (bind _output_get_2 (Variables|PlayerControlStatus|SetWasPlayerControlled false)))))

(event Custom|UpdateCameraValues
  (bind _returnvalue (Class|RuntimeBlueprintFunctionLibrary|ToConfigProperty(ModConfiguration) "/BetterVehicleCamera/Config/BetterVehicleCamera_Config.BetterVehicleCamera_Config_C"))
  (bind _mainsettingscategory (Variables|Default|GetMainSettingsCategory))
  (bind _ownerspringarm (Variables|OwnerReferences|GetOwnerSpringArm))
  (bind _asbp_config_property_section (Utilities|Casting|CastToBP_ConfigPropertySection _returnvalue))
  (bind _returnvalue_2 (Class|RuntimeBlueprintFunctionLibrary|ToConfigProperty(ConfigPropertySection) _asbp_config_property_section _mainsettingscategory))
  (bind _asconfig_property_section (Utilities|Casting|CastToConfigPropertySection _returnvalue_2))
  (bind _returnvalue_3 (Class|RuntimeBlueprintFunctionLibrary|ToConfigProperty(ConfigPropertySection) _asconfig_property_section "SpringArmPosition"))
  (bind _returnvalue_4 (Class|RuntimeBlueprintFunctionLibrary|ToConfigProperty(ConfigPropertySection) _asconfig_property_section "SpringArmLag"))
  (bind _returnvalue_5 (Class|RuntimeBlueprintFunctionLibrary|ToConfigProperty(ConfigPropertySection) _asconfig_property_section "CameraPosition"))
  (bind _asconfig_property_section_2 (Utilities|Casting|CastToConfigPropertySection _returnvalue_3))
  (bind _asconfig_property_section_3 (Utilities|Casting|CastToConfigPropertySection _returnvalue_4))
  (bind _asconfig_property_section_4 (Utilities|Casting|CastToConfigPropertySection _returnvalue_5))
  ;[1 1 1] Update Camera Position when settings changed
  (Variables|/Script/Engine.SpringArmComponent|SetbEnableCameraLag _ownerspringarm (Class|RuntimeBlueprintFunctionLibrary|ToBoolean(ConfigProperty) (Class|RuntimeBlueprintFunctionLibrary|ToConfigProperty(ConfigPropertySection) _asconfig_property_section_3 "SpringArmEnableCameraLag")))
  (Variables|/Script/Engine.SpringArmComponent|SetbEnableCameraRotationLag _ownerspringarm (Class|RuntimeBlueprintFunctionLibrary|ToBoolean(ConfigProperty) (Class|RuntimeBlueprintFunctionLibrary|ToConfigProperty(ConfigPropertySection) _asconfig_property_section_3 "SpringArmEnableCameraRotationLag")))
  (Variables|/Script/Engine.SpringArmComponent|SetCameraLagSpeed _ownerspringarm (Class|RuntimeBlueprintFunctionLibrary|ToFloat(ConfigProperty) (Class|RuntimeBlueprintFunctionLibrary|ToConfigProperty(ConfigPropertySection) _asconfig_property_section_3 "SpringArmCameraLagSpeed")))
  (Variables|/Script/Engine.SpringArmComponent|SetCameraRotationLagSpeed _ownerspringarm (Class|RuntimeBlueprintFunctionLibrary|ToFloat(ConfigProperty) (Class|RuntimeBlueprintFunctionLibrary|ToConfigProperty(ConfigPropertySection) _asconfig_property_section_3 "SpringArmCameraRotationLagSpeed")))
  (Variables|/Script/Engine.SpringArmComponent|SetCameraLagMaxDistance _ownerspringarm (Class|RuntimeBlueprintFunctionLibrary|ToFloat(ConfigProperty) (Class|RuntimeBlueprintFunctionLibrary|ToConfigProperty(ConfigPropertySection) _asconfig_property_section_3 "SpringArmCameraLagMaxDistance")))
  (Variables|/Script/Engine.SpringArmComponent|SetTargetArmLength _ownerspringarm (Class|RuntimeBlueprintFunctionLibrary|ToFloat(ConfigProperty) (Class|RuntimeBlueprintFunctionLibrary|ToConfigProperty(ConfigPropertySection) _asconfig_property_section_2 "SpringArmLength")))
  (Variables|/Script/Engine.SpringArmComponent|SetSocketOffset _ownerspringarm (+ (Variables|CameraBaseValues|GetSpringArmBaseSocketOffset) (Math|Vector|MakeVector (Class|RuntimeBlueprintFunctionLibrary|ToFloat(ConfigProperty) (Class|RuntimeBlueprintFunctionLibrary|ToConfigProperty(ConfigPropertySection) _asconfig_property_section_2 "SpringArmX")) (Class|RuntimeBlueprintFunctionLibrary|ToFloat(ConfigProperty) (Class|RuntimeBlueprintFunctionLibrary|ToConfigProperty(ConfigPropertySection) _asconfig_property_section_2 "SpringArmY")) (Class|RuntimeBlueprintFunctionLibrary|ToFloat(ConfigProperty) (Class|RuntimeBlueprintFunctionLibrary|ToConfigProperty(ConfigPropertySection) _asconfig_property_section_2 "SpringArmZ")))))
  (Transformation|SetRelativeLocationAndRotation _ownerspringarm (+ (Variables|CameraBaseValues|GetSpringArmBaseLocation) (Math|Vector|MakeVector (Class|RuntimeBlueprintFunctionLibrary|ToFloat(ConfigProperty) (Class|RuntimeBlueprintFunctionLibrary|ToConfigProperty(ConfigPropertySection) _asconfig_property_section_4 "CameraX")) (Class|RuntimeBlueprintFunctionLibrary|ToFloat(ConfigProperty) (Class|RuntimeBlueprintFunctionLibrary|ToConfigProperty(ConfigPropertySection) _asconfig_property_section_4 "CameraY")) (Class|RuntimeBlueprintFunctionLibrary|ToFloat(ConfigProperty) (Class|RuntimeBlueprintFunctionLibrary|ToConfigProperty(ConfigPropertySection) _asconfig_property_section_4 "CameraZ")))) (Math|Rotator|CombineRotators (Variables|CameraBaseValues|GetSpringArmBaseRotation) (Math|Rotator|MakeRotator 0.0 (Class|RuntimeBlueprintFunctionLibrary|ToFloat(ConfigProperty) (Class|RuntimeBlueprintFunctionLibrary|ToConfigProperty(ConfigPropertySection) (.AsConfig%20Property%20Section (Utilities|Casting|CastToConfigPropertySection (Class|RuntimeBlueprintFunctionLibrary|ToConfigProperty(ConfigPropertySection) _asconfig_property_section "SpringArmPosition"))) "SpringArmPitch")) 0.0)) false true)
  (Transformation|SetRelativeLocationAndRotation (Variables|OwnerReferences|GetOwnerCamera) "0, 0, 0" (Math|Rotator|CombineRotators (Variables|CameraBaseValues|GetCameraBaseRotation) (Math|Rotator|MakeRotator 0.0 (Class|RuntimeBlueprintFunctionLibrary|ToFloat(ConfigProperty) (Class|RuntimeBlueprintFunctionLibrary|ToConfigProperty(ConfigPropertySection) (.AsConfig%20Property%20Section (Utilities|Casting|CastToConfigPropertySection (Class|RuntimeBlueprintFunctionLibrary|ToConfigProperty(ConfigPropertySection) _asconfig_property_section "CameraPosition"))) "CameraPitch")) 0.0)) false true)
  (CallFunction|ResetCameraZoom))

(event Input|EnhancedActionEvents|EnhancedInputActionIA_BetterVehicleCamera_ZoomIn
  (params (ActionValue :type Boolean) (ElapsedSeconds :type Float%20%28double-precision%29) (TriggeredSeconds :type Float%20%28double-precision%29) (InputAction :type Input%20Action%20Object%20Reference :default "/BetterVehicleCamera/Input/IA_BetterVehicleCamera_ZoomIn.IA_BetterVehicleCamera_ZoomIn"))
  (bind _returnvalue (Class|RuntimeBlueprintFunctionLibrary|ToConfigProperty(ModConfiguration) "/BetterVehicleCamera/Config/BetterVehicleCamera_Config.BetterVehicleCamera_Config_C"))
  (bind _asbp_config_property_section (Utilities|Casting|CastToBP_ConfigPropertySection _returnvalue))
  (bind _returnvalue_2 (Class|RuntimeBlueprintFunctionLibrary|ToConfigProperty(ConfigPropertySection) _asbp_config_property_section "ScrollToZoomSettings"))
  (bind _asconfig_property_section (Utilities|Casting|CastToConfigPropertySection _returnvalue_2))
  ;[1 1 1] Zoom in if zoom active
  (:Started
    (if (Class|RuntimeBlueprintFunctionLibrary|ToBoolean(ConfigProperty) (Class|RuntimeBlueprintFunctionLibrary|ToConfigProperty(ConfigPropertySection) _asconfig_property_section "ScrollToZoomEnabled")) :!label _label
      (Variables|CameraZoom|SetCameraZoom (Math|Float|Clamp(Float) (- (Variables|CameraZoom|GetCameraZoom) (Class|RuntimeBlueprintFunctionLibrary|ToFloat(ConfigProperty) (Class|RuntimeBlueprintFunctionLibrary|ToConfigProperty(ConfigPropertySection) _asconfig_property_section "ScrollToZoomStep"))) (Variables|CameraZoom|GetCameraZoomMinimum) (Variables|CameraZoom|GetCameraZoomMaximum)))
      (CallFunction|ZoomValueChanged)))
  (:Ongoing
    (goto _label)))

(event Input|EnhancedActionEvents|EnhancedInputActionIA_BetterVehicleCamera_ZoomOut
  (params (ActionValue :type Boolean) (ElapsedSeconds :type Float%20%28double-precision%29) (TriggeredSeconds :type Float%20%28double-precision%29) (InputAction :type Input%20Action%20Object%20Reference :default "/BetterVehicleCamera/Input/IA_BetterVehicleCamera_ZoomOut.IA_BetterVehicleCamera_ZoomOut"))
  (bind _returnvalue (Class|RuntimeBlueprintFunctionLibrary|ToConfigProperty(ModConfiguration) "/BetterVehicleCamera/Config/BetterVehicleCamera_Config.BetterVehicleCamera_Config_C"))
  (bind _asbp_config_property_section (Utilities|Casting|CastToBP_ConfigPropertySection _returnvalue))
  (bind _returnvalue_2 (Class|RuntimeBlueprintFunctionLibrary|ToConfigProperty(ConfigPropertySection) _asbp_config_property_section "ScrollToZoomSettings"))
  (bind _asconfig_property_section (Utilities|Casting|CastToConfigPropertySection _returnvalue_2))
  ;[1 1 1] Zoom out if zoom active
  (:Started
    (if (Class|RuntimeBlueprintFunctionLibrary|ToBoolean(ConfigProperty) (Class|RuntimeBlueprintFunctionLibrary|ToConfigProperty(ConfigPropertySection) _asconfig_property_section "ScrollToZoomEnabled")) :!label _label
      (Variables|CameraZoom|SetCameraZoom (Math|Float|Clamp(Float) (+ (Variables|CameraZoom|GetCameraZoom) (Class|RuntimeBlueprintFunctionLibrary|ToFloat(ConfigProperty) (Class|RuntimeBlueprintFunctionLibrary|ToConfigProperty(ConfigPropertySection) _asconfig_property_section "ScrollToZoomStep"))) (Variables|CameraZoom|GetCameraZoomMinimum) (Variables|CameraZoom|GetCameraZoomMaximum)))
      (CallFunction|ZoomValueChanged)))
  (:Ongoing
    (goto _label)))

(event EventBeginPlay
  ;[1 1 1] Begin Play
  (CallFunction|GetTruckReferences)
  (CallFunction|AssignUpdateEvent))

(event EventTick
  (params (DeltaSeconds :type Float%20%28single-precision%29))
  ;[1 1 1] Tick
  (CallFunction|PlayerControlBasedUpdate))